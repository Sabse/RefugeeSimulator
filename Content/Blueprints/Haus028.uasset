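; Haus028 is a Blueprint, apparently a house, that changes through timed stages, each accompanied by an explosion sound.
; On BeginPlay, three delayed steps toggle visibility on successive overlapping pairs of components 00 to 03, without propagating to children, which suggests swapping destruction states.
; Each step plays the same sound at component 00's location.
; The sequence is hardcoded, with no damage or trigger input.
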(event EventBeginPlay
  (bind _00 (Variables|Default|Get00))
  (bind _returnvalue (Transformation|GetWorldLocation _00))
  (Utilities|FlowControl|Delay 3.0)
  (Rendering|ToggleVisibility _00 false)
  (Audio|PlaySoundatLocation "/Game/StarterContent/Audio/Explosion01.Explosion01" _returnvalue)
  (Utilities|FlowControl|Delay 3.0)
  (Rendering|ToggleVisibility (Variables|Default|Get01) false)
  (Audio|PlaySoundatLocation "/Game/StarterContent/Audio/Explosion01.Explosion01" _returnvalue)
  (Utilities|FlowControl|Delay 3.0)
  (Rendering|ToggleVisibility (Variables|Default|Get02) false)
  (Audio|PlaySoundatLocation "/Game/StarterContent/Audio/Explosion01.Explosion01" _returnvalue))

(fn ConstructionScript)