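; BP_Haus001_anders is a house actor that can appear in a destroyed state.
; Its construction script fills a Meshes array with components 00 and 01, then removes 00 through DestroyFull if MainInstance flags the city as destroyed.
; DestroyOnce removes the same component at index zero, but its index increment is unconnected and nothing here calls it.
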(event EventBeginPlay)

(fn ConstructionScript
  (CallFunction|BuildArray)
  (bind _asmain_instance (Utilities|Casting|CastToMainInstance (Game|GetGameInstance)))
  (if (Variables|/Game/Blueprints/MainInstance.MainInstance_C|GetDestroyedCity _asmain_instance)
    (CallFunction|DestroyFull)))

(fn DestroyFull
  (Components|DestroyComponent (Variables|Default|Get00)))

(fn DestroyOnce
  (switch int (Variables|Default|GetCurrentIndex)
    (:0
      (Components|DestroyComponent (Variables|Default|Get00)))))

(fn BuildArray
  (bind _meshes (Variables|Default|GetMeshes))
  (Utilities|Array|Add _meshes (Variables|Default|Get00))
  (Utilities|Array|Add _meshes (Variables|Default|Get01)))