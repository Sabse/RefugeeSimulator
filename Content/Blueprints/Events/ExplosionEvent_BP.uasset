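; ExplosionEvent_BP is an event actor that sets off an explosion when another actor overlaps it.
; The overlap fires only while IsActive is true and IsTriggered is false, though this graph never sets either flag.
; It plays the explosion sound, toggles the explosion and fire components, and fires a radial force impulse.
; Because the effects are toggled rather than activated, a repeated overlap can switch them back off.
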(event Collision|EventActorBeginOverlap
  (params (OtherActor :type Actor%20Object%20Reference))
  (if (Variables|Default|GetisActive)
    (if (not (Variables|Default|GetisTriggered))
      (Class|FMODAudioComponent|Play (Variables|Default|GetExplosionSound))
      (Components|Activation|ToggleActive (Variables|Default|GetExplosion))
      (Class|RadialForceComponent|FireImpulse (Variables|Default|GetRadialForce)))))

(fn ConstructionScript)