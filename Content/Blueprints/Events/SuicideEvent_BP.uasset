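; SuicideEvent_BP is an overlap-triggered scripted event that shows an animated suicide figure with a scream.
; When an actor overlaps it while IsActive is set and IsTriggered is not, it plays the audio and a non-looping skeletal animation.
; The WalkDistance timeline simultaneously moves the whole actor by a track offset from the location stored at BeginPlay.
; The graph checks IsTriggered but never sets it.
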(event Collision|EventActorBeginOverlap
  (params (OtherActor :type Actor%20Object%20Reference))
  (if (Variables|Default|GetisActive)
    (if (not (Variables|Default|GetisTriggered))
      (Class|FMODAudioComponent|Play (Variables|Default|Getscream%20fap))
      (Components|Animation|PlayAnimation (Variables|Default|GetSuicideVikSmoothEdge3DS) "/Game/Meshes/SuicideVikSmoothEdge3DS_Anim.SuicideVikSmoothEdge3DS_Anim" false)
      (bind _newtrack_2 (Timeline|Walk%20Distance Play)
        (:Update
          (Transformation|SetActorLocation (+ _newtrack_2 (Variables|Default|GetEvent%20Initial%20Location)) false false))))))

(event EventBeginPlay
  (Variables|Default|SetEvent%20Initial%20Location (Transformation|GetActorLocation)))

(fn ConstructionScript)