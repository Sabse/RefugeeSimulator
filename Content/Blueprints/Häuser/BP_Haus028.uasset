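; BP_Haus028 is a house Blueprint that shows different destruction states by swapping the static mesh on MainMesh from its Meshes array.
; The construction script applies the mesh at DestructionLevel, resetting it to zero in any level other than MainLevel_Destroyed.
; DestroyRandom picks any mesh from the array, while DestroyOnce advances a separate CurrentIndex one step until the last mesh.
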(event EventBeginPlay)

(fn ConstructionScript
  (bind _returnvalue (Game|GetCurrentLevelName true))
  (if (Utilities|Enum|Equal(Enum) _returnvalue "MainLevel_Destroyed")
    _
    (else
      (Variables|Destruction|SetDestructionLevel 0)))
  (Components|StaticMesh|SetStaticMesh (Variables|Default|GetMainMesh) (Utilities|Array|Get(acopy) (Variables|Default|GetMeshes) (Variables|Destruction|GetDestructionLevel))))

(fn DestroyRandom
  (bind _meshes (Variables|Default|GetMeshes))
  (Components|StaticMesh|SetStaticMesh (Variables|Default|GetMainMesh) (Utilities|Array|Get(acopy) _meshes (Math|Random|RandomIntegerinRange 0 (Utilities|Array|LastIndex _meshes)))))

(fn DestroyOnce
  (bind _meshes (Variables|Default|GetMeshes))
  (if (< (Variables|Default|GetCurrentIndex) (Utilities|Array|LastIndex _meshes))
    (Components|StaticMesh|SetStaticMesh (Variables|Default|GetMainMesh) (Utilities|Array|Get(acopy) _meshes (+ (Variables|Default|GetCurrentIndex) 1)))
    (Variables|Default|SetCurrentIndex (+ (Variables|Default|GetCurrentIndex) 1))))