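; BP_Haus005 is a destructible house that swaps its static mesh through an array of destruction stages.
; The construction script shows the fully destroyed stage if the MainInstance game instance flags DestroyedCity, otherwise the first mesh.
; DestroyOnce advances CurrentIndex and the mesh by one stage until the last one.
; DestroyFull repeats DestroyOnce to reach the final stage; BeginPlay does nothing.
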(event EventBeginPlay)

(fn ConstructionScript
  (bind _asmain_instance (Utilities|Casting|CastToMainInstance (Game|GetGameInstance))
    (:then
      (if (Variables|/Game/Blueprints/MainInstance.MainInstance_C|GetDestroyedCity _asmain_instance)
        (CallFunction|DestroyFull)
        (else
          (Components|StaticMesh|SetStaticMesh (Variables|Default|GetMainMesh) (Utilities|Array|Get(acopy) (Variables|Default|GetMeshes)) :!label _label))))
    (:CastFailed
      (goto _label))))

(fn DestroyFull
  (bind _meshes (Variables|Default|GetMeshes))
  (bind _returnvalue (Utilities|Array|LastIndex _meshes))
  (for _index (range 0 (- _returnvalue 1))
    (CallFunction|DestroyOnce))
  (Variables|Default|SetCurrentIndex _returnvalue))

(fn DestroyOnce
  (bind _meshes (Variables|Default|GetMeshes))
  (if (< (Variables|Default|GetCurrentIndex) (Utilities|Array|LastIndex _meshes))
    (Components|StaticMesh|SetStaticMesh (Variables|Default|GetMainMesh) (Utilities|Array|Get(acopy) _meshes (+ (Variables|Default|GetCurrentIndex) 1)))
    (Variables|Default|SetCurrentIndex (+ (Variables|Default|GetCurrentIndex) 1))))