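; BP_Haus002 is a house Blueprint that shows intact or damaged states by swapping the static mesh on MainMesh from a Meshes array.
; Its construction script picks a random damaged mesh when MainInstance flags DestroyedCity and the house is Destructible, otherwise the first mesh.
; DestroyOnce advances CurrentIndex one damage stage at a time up to the last mesh.
; The random pick leaves CurrentIndex untouched.
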(event EventBeginPlay)

(fn ConstructionScript
  (bind _asmain_instance (Utilities|Casting|CastToMainInstance (Game|GetGameInstance))
    (:then
      (if (Variables|/Game/Blueprints/MainInstance.MainInstance_C|GetDestroyedCity _asmain_instance)
        (if (Variables|Default|GetDestructible)
          (CallFunction|DestroyRandom)
          (else
            (Components|StaticMesh|SetStaticMesh (Variables|Default|GetMainMesh) (Utilities|Array|Get(acopy) (Variables|Default|GetMeshes)) :!label _label)))
        (else
          (goto _label))))
    (:CastFailed
      (goto _label))))

(fn DestroyRandom
  (bind _meshes (Variables|Default|GetMeshes))
  (Components|StaticMesh|SetStaticMesh (Variables|Default|GetMainMesh) (Utilities|Array|Get(acopy) _meshes (Math|Random|RandomIntegerinRange 1 (Utilities|Array|LastIndex _meshes)))))

(fn DestroyOnce
  (bind _meshes (Variables|Default|GetMeshes))
  (if (< (Variables|Default|GetCurrentIndex) (Utilities|Array|LastIndex _meshes))
    (Components|StaticMesh|SetStaticMesh (Variables|Default|GetMainMesh) (Utilities|Array|Get(acopy) _meshes (+ (Variables|Default|GetCurrentIndex) 1)))
    (Variables|Default|SetCurrentIndex (+ (Variables|Default|GetCurrentIndex) 1))))