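; Protagonist Blueprint that lets key presses arm or disarm four scripted events (explosion, suicide, scream, shots) and toggle a movement flag.
; An armed event fires once on actor overlap, locking its toggle and sending the same marker byte through SendByte for all four.
; Every toggle and trigger goes through OnEventTriggered to a C++ timestamped log and console print, with German action labels.
; BeginPlay adds an icon widget to the viewport.
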(event OnActorBeginOverlap(ExplosionEvent)
  (params (OtherActor :type Actor%20Object%20Reference))
  (bind _explosionevent (Variables|Event|GetExplosionEvent))
  ;[1 1 1] If certain event is triggered, deactivate input
  (if (Variables|/Game/Blueprints/Events/ExplosionEvent_BP.ExplosionEvent_BP_C|GetisActive _explosionevent)
    (if (not (Variables|/Game/Blueprints/Events/ExplosionEvent_BP.ExplosionEvent_BP_C|GetisTriggered _explosionevent))
      (Variables|/Game/Blueprints/Events/ExplosionEvent_BP.ExplosionEvent_BP_C|SetisTriggered _explosionevent true)
      ;[1 1 1] Call C++ Log Function
      (CallFunction|OnEventTriggered "Explosion Event " "ausgelöst")
      ;[1 1 1] Send Marker
      (Class|EKGCommunicationActor|SendByte 10))))

(event OnActorBeginOverlap(SuicideEvent)
  (params (OtherActor :type Actor%20Object%20Reference))
  (bind _suicideevent (Variables|Event|GetSuicideEvent))
  ;[1 1 1] If certain event is triggered, deactivate input
  (if (Variables|/Game/Blueprints/Events/SuicideEvent_BP.SuicideEvent_BP_C|GetisActive _suicideevent)
    (if (not (Variables|/Game/Blueprints/Events/SuicideEvent_BP.SuicideEvent_BP_C|GetisTriggered _suicideevent))
      (Variables|/Game/Blueprints/Events/SuicideEvent_BP.SuicideEvent_BP_C|SetisTriggered _suicideevent true)
      ;[1 1 1] Call C++ Log Function
      (CallFunction|OnEventTriggered "Suicide Event " "ausgelöst")
      ;[1 1 1] Send Marker
      (Class|EKGCommunicationActor|SendByte 10))))

(event OnActorBeginOverlap(ScreamEvent)
  (params (OtherActor :type Actor%20Object%20Reference))
  (bind _screamevent (Variables|Event|GetScreamEvent))
  ;[1 1 1] If certain event is triggered, deactivate input
  (if (Variables|/Game/Blueprints/Events/ScreamEvent_BP.ScreamEvent_BP_C|GetisActive _screamevent)
    (if (not (Variables|/Game/Blueprints/Events/ScreamEvent_BP.ScreamEvent_BP_C|GetisTriggered _screamevent))
      (Variables|/Game/Blueprints/Events/ScreamEvent_BP.ScreamEvent_BP_C|SetisTriggered _screamevent true)
      ;[1 1 1] Call C++ Log Function
      (CallFunction|OnEventTriggered "Scream Event " "ausgelöst")
      ;[1 1 1] Send Marker
      (Class|EKGCommunicationActor|SendByte 10))))

(event OnActorBeginOverlap(ShotsEvent)
  (params (OtherActor :type Actor%20Object%20Reference))
  (bind _shotsevent (Variables|Event|GetShotsEvent))
  ;[1 1 1] If certain event is triggered, deactivate input
  (if (Variables|/Game/Blueprints/Events/ShotsEvent_BP.ShotsEvent_BP_C|GetisActive _shotsevent)
    (if (not (Variables|/Game/Blueprints/Events/ShotsEvent_BP.ShotsEvent_BP_C|GetisTriggered _shotsevent))
      (Variables|/Game/Blueprints/Events/ShotsEvent_BP.ShotsEvent_BP_C|SetisTriggered _shotsevent true)
      ;[1 1 1] Call C++ Log Function
      (CallFunction|OnEventTriggered "Shots Event " "ausgelöst")
      ;[1 1 1] Send Marker
      (Class|EKGCommunicationActor|SendByte 10))))

(event Custom|OnEventTriggered
  (params (EventName :type String) (Action :type String))
  ;[1 1 1] C++ log function call & Console Output
  (Class|RefugeeSimulatorProtagonist|LogEvent (Utilities|Time|GetGameTimeinSeconds) EventName Action)
  (Development|PrintText 0 (Utilities|Text|ToText(String) (Utilities|String|Append EventName Action)) false))

(event EventBeginPlay
  ;[1 1 1] Setup Icon Widget to view in Viewport and get Variables to interact
  (bind _returnvalue (UserInterface|CreateWidget "/Game/GUI/Widgets/IconWidget.IconWidget_C" (Game|GetPlayerController 0)))
  (UserInterface|Viewport|AddtoViewport _returnvalue 0))

(event Input|ActionEvents|InputActionScream
  (params (Key :type Key%20Structure :default "AnyKey"))
  (bind _screamevent (Variables|Event|GetScreamEvent))
  ;[1 1 1] Scream Event Set Active
  (:Pressed
    (if (not (Variables|/Game/Blueprints/Events/ScreamEvent_BP.ScreamEvent_BP_C|GetisTriggered _screamevent))
      (if (Variables|/Game/Blueprints/Events/ScreamEvent_BP.ScreamEvent_BP_C|GetisActive _screamevent)
        (Variables|/Game/Blueprints/Events/ScreamEvent_BP.ScreamEvent_BP_C|SetisActive (Variables|Event|GetScreamEvent) false)
        ;[1 1 1] Call C++ Log Function
        (CallFunction|OnEventTriggered "Scream Event " "deaktiviert")
        (else
          (Variables|/Game/Blueprints/Events/ScreamEvent_BP.ScreamEvent_BP_C|SetisActive (Variables|Event|GetScreamEvent) true)
          (CallFunction|OnEventTriggered "Scream Event " "aktiviert"))))))

(event Input|ActionEvents|InputActionShots
  (params (Key :type Key%20Structure :default "AnyKey"))
  (bind _shotsevent (Variables|Event|GetShotsEvent))
  ;[1 1 1] Shots Event Set Active
  (:Pressed
    (if (not (Variables|/Game/Blueprints/Events/ShotsEvent_BP.ShotsEvent_BP_C|GetisTriggered _shotsevent))
      (if (Variables|/Game/Blueprints/Events/ShotsEvent_BP.ShotsEvent_BP_C|GetisActive _shotsevent)
        (Variables|/Game/Blueprints/Events/ShotsEvent_BP.ShotsEvent_BP_C|SetisActive (Variables|Event|GetShotsEvent) false)
        ;[1 1 1] Call C++ Log Function
        (CallFunction|OnEventTriggered "Shots Event " "deaktiviert")
        (else
          (Variables|/Game/Blueprints/Events/ShotsEvent_BP.ShotsEvent_BP_C|SetisActive (Variables|Event|GetShotsEvent) true)
          (CallFunction|OnEventTriggered "Shots event " "aktiviert"))))))

(event Input|ActionEvents|InputActionMovement
  (params (Key :type Key%20Structure :default "AnyKey"))
  ;[1 1 1] Enable/Disable play movement by pressing M
  (:Pressed
    (if (Variables|Default|GetmovementEnabled)
      (Variables|Default|SetmovementEnabled false)
      ;[1 1 1] Call C++ Log Function
      (CallFunction|OnEventTriggered "Movement " "deaktiviert")
      (else
        (Variables|Default|SetmovementEnabled true)
        (CallFunction|OnEventTriggered "Movement " "aktiviert")))))

(event Input|ActionEvents|InputActionExplosion
  (params (Key :type Key%20Structure :default "AnyKey"))
  (bind _explosionevent (Variables|Event|GetExplosionEvent))
  ;[1 1 1] Explosion Event Set Active
  (:Pressed
    (if (not (Variables|/Game/Blueprints/Events/ExplosionEvent_BP.ExplosionEvent_BP_C|GetisTriggered _explosionevent))
      (if (Variables|/Game/Blueprints/Events/ExplosionEvent_BP.ExplosionEvent_BP_C|GetisActive _explosionevent)
        (Variables|/Game/Blueprints/Events/ExplosionEvent_BP.ExplosionEvent_BP_C|SetisActive (Variables|Event|GetExplosionEvent) false)
        ;[1 1 1] Call C++ Log Function
        (CallFunction|OnEventTriggered "Explosion Event " "deaktiviert")
        (else
          (Variables|/Game/Blueprints/Events/ExplosionEvent_BP.ExplosionEvent_BP_C|SetisActive (Variables|Event|GetExplosionEvent) true)
          (CallFunction|OnEventTriggered "Explosion Event " "aktiviert"))))))

(event Input|ActionEvents|InputActionSuicide
  (params (Key :type Key%20Structure :default "AnyKey"))
  (bind _suicideevent (Variables|Event|GetSuicideEvent))
  ;[1 1 1] Suicide Event Set Active
  (:Pressed
    (if (not (Variables|/Game/Blueprints/Events/SuicideEvent_BP.SuicideEvent_BP_C|GetisTriggered _suicideevent))
      (if (Variables|/Game/Blueprints/Events/SuicideEvent_BP.SuicideEvent_BP_C|GetisActive _suicideevent)
        (Variables|/Game/Blueprints/Events/SuicideEvent_BP.SuicideEvent_BP_C|SetisActive (Variables|Event|GetSuicideEvent) false)
        ;[1 1 1] Call C++ Log Function
        (CallFunction|OnEventTriggered "Suicide Event " "deaktiviert")
        (else
          (Variables|/Game/Blueprints/Events/SuicideEvent_BP.SuicideEvent_BP_C|SetisActive (Variables|Event|GetSuicideEvent) true)
          (CallFunction|OnEventTriggered "Suicide Event " "aktiviert"))))))

(fn ConstructionScript)